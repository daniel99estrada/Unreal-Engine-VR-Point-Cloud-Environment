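; Actor that displays a LiDAR point cloud and carries a map cursor for positioning within it, linked to the VR pawn.
; Assigning a cloud sets the spring arm length to the largest absolute XY bound and returns the cloud to the world origin.
; The actor itself moves to pawn map or given XY positions at cursor height.
; The cursor update clamps XY to cloud bounds, but its speed is multiplied by zero.
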(event Custom|Set%20Spring%20Arm%20Length
  (bind _lidarpointcloud (Variables|Default|GetLidarPointCloud))
  (bind _pointcloud (Variables|/Script/LidarPointCloudRuntime.LidarPointCloudComponent|GetPointCloud _lidarpointcloud))
  (bind _returnvalue (Class|LidarPointCloud|GetBounds _pointcloud false))
  (Variables|/Script/Engine.SpringArmComponent|SetTargetArmLength (Variables|Default|GetSpringArm) (Math|Float|Max(Float) (Math|Float|Max(Float) (Math|Float|Absolute(Float) (.x (.min _returnvalue))) (Math|Float|Absolute(Float) (.x (.max _returnvalue)))) (Math|Float|Max(Float) (Math|Float|Absolute(Float) (.y (.min _returnvalue))) (Math|Float|Absolute(Float) (.y (.max _returnvalue)))))))

(event Custom|Set%20Location%20In%20Map
  (bind _vr_pawn (Variables|Default|GetVR%20Pawn))
  (bind _maplocation (Variables|/Game/VRTemplate/Blueprints/VRPawn.VRPawn_C|GetMapLocation _vr_pawn))
  ;[1 1 1] Set Location In Map
  (Transformation|SetActorLocation (Math|Vector|MakeVector (.x _maplocation) (.y _maplocation) (.z (Transformation|GetWorldLocation (Variables|Default|GetCursor)))) false false))

(fn ConstructionScript)

(fn GetArea
  (return (Class|LidarPointCloud|GetBounds (Class|LidarPointCloudComponent|GetPointCloud (Variables|Default|GetLidarPointCloud)) false)))

(fn SetPointCloudFile
  (params (InPointCloud :type Lidar%20Point%20Cloud%20Object%20Reference))
  (bind _lidarpointcloud (Variables|Default|GetLidarPointCloud))
  (Class|LidarPointCloudComponent|SetPointCloud _lidarpointcloud InPointCloud)
  (CallFunction|SetSpringArmLength)
  (Transformation|SetWorldLocation _lidarpointcloud "0, 0, 0" false false))

(fn UpdateCursorLocation
  (bind _returnvalue (Transformation|GetActorLocation))
  (bind _lidarpointcloud (Variables|Default|GetLidarPointCloud))
  (bind _pointcloud (Variables|/Script/LidarPointCloudRuntime.LidarPointCloudComponent|GetPointCloud _lidarpointcloud))
  (bind _returnvalue_2 (Class|LidarPointCloud|GetBounds _pointcloud false))
  (Transformation|SetActorLocation (Math|Vector|MakeVector (Math|Float|Clamp(Float) (+ (* 0.0 (Variables|Default|GetSpeed)) (.x _returnvalue)) (.x (.min _returnvalue_2)) (.x (.max _returnvalue_2))) (Math|Float|Clamp(Float) (+ (* (Variables|Default|GetSpeed) 0.0) (.y _returnvalue)) (.y (.min _returnvalue_2)) (.y (.max _returnvalue_2))) (.z _returnvalue)) false false))

(fn GetCursorLocation
  (return (Transformation|GetWorldLocation (Variables|Default|GetCursor))))

(fn EnableCursor
  (params (bNewVisibility :type Boolean))
  (Rendering|SetVisibility (Variables|Default|GetCursor) bNewVisibility false))

(fn SetCursorLocation
  (params (NewParam :type Vector))
  (Transformation|SetActorLocation (Math|Vector|MakeVector (.x NewParam) (.y NewParam) (.z (Transformation|GetWorldLocation (Variables|Default|GetCursor)))) false false))