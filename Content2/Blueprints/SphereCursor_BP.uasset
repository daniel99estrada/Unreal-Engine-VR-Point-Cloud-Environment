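; SphereCursor_BP is a sphere cursor actor that moves horizontally within the bounds of the VR pawn's active point cloud.
; Custom events show or hide the sphere along with its collision and tick, or place it at the pawn's MapLocation at CursorHeight.
; UpdateSphereLocation applies speed-scaled 2D input with X and Y swapped, clamps the result to the cloud's XY bounds and keeps Z unchanged.
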(event Custom|Enable%20Cursor%20Visual
  (bind _sphere (Variables|Default|GetSphere))
  ;[1 1 1] Make Sphere Visible
  (Rendering|SetVisibility _sphere true false)
  (Collision|SetCollisionEnabled _sphere "QueryAndPhysics")
  (Components|Tick|SetComponentTickEnabled _sphere true))

(event Custom|Disable%20Cursor%20Visual
  (bind _sphere (Variables|Default|GetSphere))
  ;[1 1 1] Make Sphere Invisible
  (Rendering|SetVisibility _sphere false false)
  (Collision|SetCollisionEnabled _sphere "NoCollision")
  (Components|Tick|SetComponentTickEnabled _sphere false))

(event Custom|Set%20Location%20In%20Map
  (bind _vrpawn (Variables|Default|GetVRpawn))
  (bind _maplocation (Variables|/Game/VRTemplate/Blueprints/VRPawn.VRPawn_C|GetMapLocation _vrpawn))
  ;[1 1 1] Set Location In Map
  (Transformation|SetActorLocation (Math|Vector|MakeVector (.x _maplocation) (.y _maplocation) (Variables|Default|GetCursor%20height)) false false))

(event EventBeginPlay
  (Development|PrintString "Hello"))

(fn ConstructionScript)

(fn UpdateSphereLocation
  (params (NewParam :type Vector%202D%20Structure))
  (bind _returnvalue (Transformation|GetActorLocation))
  (bind _vrpawn (Variables|Default|GetVRpawn))
  (bind _active_point_cloud (Variables|/Game/VRTemplate/Blueprints/VRPawn.VRPawn_C|GetActive%20Point%20Cloud _vrpawn))
  (bind _returnvalue_2 (Class|LidarPointCloud|GetBounds _active_point_cloud false))
  (Transformation|SetActorLocation (Math|Vector|MakeVector (Math|Float|Clamp(Float) (+ (* (.y NewParam) (Variables|Default|GetSpeed)) (.x _returnvalue)) (.x (.min _returnvalue_2)) (.x (.max _returnvalue_2))) (Math|Float|Clamp(Float) (+ (* (.x NewParam) (Variables|Default|GetSpeed)) (.y _returnvalue)) (.y (.min _returnvalue_2)) (.y (.max _returnvalue_2))) (.z _returnvalue)) false false))